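; Walkable AI character that drives movement from four needs: food, water, mental and physical.
; It picks a random walk speed on BeginPlay and drains every need on Tick.
; While idle, the first depleted need in that priority order issues an AIMoveTo with no target set, refills immediately and locks out new moves until it ends.
; A random navmesh wander move is present but disconnected.
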(event EventBeginPlay
  (bind _output_get (Variables|Default|SetWalk_spd (Math|Random|RandomFloatinRange 1e+02 4.5e+02)))
  (Variables|/Script/Engine.CharacterMovementComponent|SetMaxWalkSpeed (Variables|Character|GetCharacterMovement) _output_get))

(event EventTick
  (params (DeltaSeconds :type Float%20%28single-precision%29))
  ;[1 1 1] Wander
  (Variables|Default|SetFood (- (Variables|Default|GetFood) DeltaSeconds))
  (Variables|Default|SetWater (- (Variables|Default|GetWater) DeltaSeconds))
  (Variables|Default|SetMental (- (Variables|Default|GetMental) DeltaSeconds))
  (Variables|Default|SetPhysical (- (Variables|Default|GetPhysical) DeltaSeconds))
  (if (not (Variables|Default|Getiswalking?))
    (if (<= (Variables|Default|GetFood) 0.0)
      (AI|AIMoveTo 0 "0, 0, 0" 0 5.0 false
        (:then
          (Variables|Default|SetFood 1e+01)
          (Variables|Default|Setiswalking? true :!label _label))
        (:OnSuccess
          (Variables|Default|Setiswalking? false :!label _label_2))
        (:OnFail
          (goto _label_2)))
      (elif (<= (Variables|Default|GetWater) 0.0)
        (AI|AIMoveTo 0 "0, 0, 0" 0 5.0 false
          (:then
            (Variables|Default|SetWater 1e+01)
            (goto _label))
          (:OnSuccess
            (goto _label_2))
          (:OnFail
            (goto _label_2)))
        (elif (<= (Variables|Default|GetMental) 0.0)
          (AI|AIMoveTo 0 "0, 0, 0" 0 5.0 false
            (:then
              (Variables|Default|SetMental 1e+01)
              (goto _label))
            (:OnSuccess
              (goto _label_2))
            (:OnFail
              (goto _label_2)))
          (elif (<= (Variables|Default|GetPhysical) 0.0)
            (AI|AIMoveTo 0 "0, 0, 0" 0 5.0 false
              (:then
                (Variables|Default|SetPhysical 1e+01)
                (goto _label))
              (:OnSuccess
                (goto _label_2))
              (:OnFail
                (goto _label_2)))))))))

(fn ConstructionScript)