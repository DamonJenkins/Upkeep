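; Wander is a character that roams to random points on the navmesh.
; On BeginPlay it picks a random walk speed and applies it to its CharacterMovement.
; Tick starts an AI MoveTo toward a random navigable point within MoveRange of its location whenever it is not already walking.
; The Iswalking flag blocks new requests until the move succeeds or fails, so wandering repeats continuously.
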(event EventBeginPlay
  (bind _output_get (Variables|Default|SetWalk_spd (Math|Random|RandomFloatinRange 1e+02 4.5e+02)))
  (Variables|/Script/Engine.CharacterMovementComponent|SetMaxWalkSpeed (Variables|Character|GetCharacterMovement) _output_get))

(event Collision|EventActorBeginOverlap
  (params (OtherActor :type Actor%20Object%20Reference)))

(event EventTick
  (params (DeltaSeconds :type Float%20%28single-precision%29))
  (if (not (Variables|Default|Getiswalking?))
    (AI|AIMoveTo self (.RandomLocation (Class|NavigationSystemV1|GetRandomPointinNavigableRadius (Transformation|GetActorLocation) (Variables|Default|GetMove_Range) 0 0)) 0 5.0 false
      (:then
        (Variables|Default|Setiswalking? true))
      (:OnSuccess
        (Variables|Default|Setiswalking? false :!label _label))
      (:OnFail
        (goto _label)))))

(fn ConstructionScript)